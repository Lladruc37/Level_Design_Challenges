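; BP_BallPendulum is a swinging ball hazard that calls EventDeath on the first-person character when the ball overlaps it.
; On BeginPlay, two timelines start alternating, one forward and one in reverse, each setting the Point component's pitch from its SwingTrack.
; Delay nodes chained from each timeline's Update, rather than Finished, start the other timeline, looping the swing on fixed timing without Tick.
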(event `self.ReceiveBeginPlay`
  (bind (_direction _swingtrack) (`Timeline|Timeline_0` :!via `PlayFromStart` :!label _label)
    (:`Update`
      (`SceneComponent.K2_SetRelativeRotation` (`self.Point`) (`KismetMathLibrary.MakeRotator` 0.0 _swingtrack) false false)
      (`KismetSystemLibrary.Delay` 2.0)
      (bind (_direction_2 _swingtrack_2) (`Timeline|Timeline_1` :!via `ReverseFromEnd`)
        (:`Update`
          (`SceneComponent.K2_SetRelativeRotation` (`self.Point`) (`KismetMathLibrary.MakeRotator` 0.0 _swingtrack_2) false false)
          (`KismetSystemLibrary.Delay` 2.0)
          (goto _label :!via `PlayFromStart`))))))

(event `self.Ball.OnComponentBeginOverlap`
  (params (OverlappedComponent :type "PrimitiveComponent Object Reference") (OtherActor :type "Actor Object Reference") (OtherComp :type "PrimitiveComponent Object Reference") (OtherBodyIndex :type Integer) (bFromSweep :type Boolean) (SweepResult :type "HitResult Structure (by ref)"))
  (bind _asbp_first_person_character (cast `/Game/FirstPerson/Blueprints/BP_FirstPersonCharacter` OtherActor))
  (`/Game/FirstPerson/Blueprints/BP_FirstPersonCharacter.EventDeath` _asbp_first_person_character))

(fn `UserConstructionScript`)